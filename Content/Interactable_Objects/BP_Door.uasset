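; BP_Door is an interactable door that toggles between open and closed each time Interact is called.
; Interact checks IsOpen and calls OpenDoor or CloseDoor, which plays or reverses the DoorAnim timeline.
; The timeline lerps the Arrow component's relative yaw between ClosedPos and OpenPos.
; Roll and pitch are fed from the Arrow's relative location X and Y, not its rotation.
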(event Custom|Open%20Door
  (bind _arrow (Variables|Default|GetArrow))
  (bind _relativelocation (Variables|/Script/Engine.SceneComponent|GetRelativeLocation _arrow))
  (Variables|Default|SetIsOpen true)
  (bind _anim (Timeline|Door%20Anim Play)
    (:Update
      (Transformation|SetRelativeRotation _arrow (Math|Rotator|MakeRotator (.x _relativelocation) (.y _relativelocation) (Math|Float|Lerp (Variables|Default|GetClosedPos) (Variables|Default|GetOpenPos) _anim)) false false))))

(event Custom|Close%20Door
  (bind _arrow (Variables|Default|GetArrow))
  (bind _relativelocation (Variables|/Script/Engine.SceneComponent|GetRelativeLocation _arrow))
  (Variables|Default|SetIsOpen false)
  (bind _anim (Timeline|Door%20Anim Reverse)
    (:Update
      (Transformation|SetRelativeRotation _arrow (Math|Rotator|MakeRotator (.x _relativelocation) (.y _relativelocation) (Math|Float|Lerp (Variables|Default|GetClosedPos) (Variables|Default|GetOpenPos) _anim)) false false))))

(event EventInteract
  (params (Instigator :type Actor%20Object%20Reference))
  (if (Variables|Default|GetIsOpen)
    (CallFunction|CloseDoor)
    (else
      (CallFunction|OpenDoor))))

(fn ConstructionScript)